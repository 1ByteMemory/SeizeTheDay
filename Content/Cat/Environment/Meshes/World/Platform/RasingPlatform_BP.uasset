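; RasingPlatform_BP is a platform actor meant to move its SMPlatform2 mesh when a SideScrollerCharacter triggers it.
; BeginPlay caches the mesh's world position as both StartLoc and Location, and stores the Box position in TargetLoc.
; An overlap-signature custom event, with no binding shown, plays a timeline that sweeps the mesh's relative location between StartLoc and Location.
; Those endpoints are identical as written, and TargetLoc is never read.
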(event `self.ReceiveBeginPlay`
  (bind _output_get (set `self.Start_Loc` (`SceneComponent.K2_GetComponentLocation` (`self.SM_Platform2`))))
  (set `self.Location` _output_get)
  (set `self.Target_Loc` (`SceneComponent.K2_GetComponentLocation` (`self.Box`)))
  (set `self.Movement speed` (`self.Movement speed`)))

(event `self.ReceiveTick`
  (params (DeltaSeconds :type "Float (single-precision)")))

(event `CustomEvent`
  (params (OverlappedComponent :type "PrimitiveComponent Object Reference") (OtherActor :type "Actor Object Reference") (OtherComp :type "PrimitiveComponent Object Reference") (OtherBodyIndex :type Integer) (bFromSweep :type Boolean) (SweepResult :type "HitResult Structure (by ref)"))
  (cast `/Game/StandardSetUpPack/Blueprints/SideScrollerCharacter` OtherActor)
  (bind (_direction _newtrack_0) (`Timeline|Timeline_1`)
    (:`Update`
      (`SceneComponent.K2_SetRelativeLocation` (`self.SM_Platform2`) (`KismetMathLibrary.VLerp` (`self.Start_Loc`) (`self.Location`) _newtrack_0) true false))))

(fn `UserConstructionScript`)
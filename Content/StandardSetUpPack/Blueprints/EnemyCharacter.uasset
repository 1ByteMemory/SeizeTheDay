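; Side-scroller melee enemy character that chases the player, deals contact damage and dies to sword hits.
; Pawn sensing starts an AI move toward any seen SideScrollerCharacter.
; Tick polls capsule overlap with the player and applies damage after a Delay, throttling it to about once per second.
; Overlaps with the player's SwordDamageField reduce Health, and Tick destroys the enemy once it is depleted.
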(event `self.ReceiveBeginPlay`
  (set `self.Health` 100.0)
  (set `self.Damage Per Tick` 20.0))

(event `self.ReceiveTick`
  (params (DeltaSeconds :type "Float (single-precision)"))
  (bind _returnvalue (`GameplayStatics.GetPlayerCharacter` 0))
  (if (<= (`self.Health`) 0.0)
    (`self.K2_DestroyActor`)
    (elif (`PrimitiveComponent.IsOverlappingActor` (`self.CapsuleComponent`) _returnvalue)
      (bind _asside_scroller_character (cast `/Game/StandardSetUpPack/Blueprints/SideScrollerCharacter` _returnvalue))
      (`KismetSystemLibrary.Delay` 1.0)
      (`/Game/StandardSetUpPack/Blueprints/SideScrollerCharacter.TakeDamage` _asside_scroller_character (`self.Damage Per Tick`)))))

(event `self.CapsuleComponent.OnComponentBeginOverlap`
  (params (OverlappedComponent :type "PrimitiveComponent Object Reference") (OtherActor :type "Actor Object Reference") (OtherComp :type "PrimitiveComponent Object Reference") (OtherBodyIndex :type Integer) (bFromSweep :type Boolean) (SweepResult :type "HitResult Structure (by ref)"))
  (bind _asside_scroller_character (cast `/Game/StandardSetUpPack/Blueprints/SideScrollerCharacter` (`GameplayStatics.GetPlayerCharacter` 0)))
  (if (== (`/Game/StandardSetUpPack/Blueprints/SideScrollerCharacter.SwordDamageField` _asside_scroller_character) OtherComp)
    (set `self.Health` (- (`self.Health`) 34.0))))

(event `self.PawnSensing.OnSeePawn`
  (params (Pawn :type "Pawn Object Reference"))
  (bind _asside_scroller_character (cast `/Game/StandardSetUpPack/Blueprints/SideScrollerCharacter` Pawn))
  (`|AIMoveTo` self (0.0 0.0 0.0) _asside_scroller_character))

(fn `UserConstructionScript`)